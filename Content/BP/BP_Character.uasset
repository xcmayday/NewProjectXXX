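; Character Blueprint that can roam as an AI between target points and takes point damage.
; After a startup delay, its fixed-point AI mode loops AIMoveTo toward FindTargetPoint, pausing after success or failure until the character is dead.
; Point damage feeds TakeDmage and draws a debug sphere at the hit location.
; Any and radial damage events are empty, with their damage logic left disconnected.
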(event `self.ReceiveBeginPlay`
  (`parent.ReceiveBeginPlay`)
  (`KismetSystemLibrary.Delay` 2.0)
  (switch `EAIModeType` (`self.AIModeType`)
    (:`AIMode_Point`
      (if (not (`self.GetIsDeadState`)) :!label _label
        (bind _movementresult (`|AIMoveTo` self (0.0 0.0 0.0) (`self.FindTargetPoint`))
          (:`OnSuccess`
            _)
          (:`OnFail`
            _))
        (`KismetSystemLibrary.Delay` 1.5)
        (goto _label)))))

(event `self.ReceiveAnyDamage`
  (params (Damage :type "Float (single-precision)") (DamageType :type "DamageType Object Reference") (InstigatedBy :type "Controller Object Reference") (DamageCauser :type "Actor Object Reference")))

(event `self.ReceiveRadialDamage`
  (params (DamageReceived :type "Float (single-precision)") (DamageType :type "DamageType Object Reference") (Origin :type "Vector Structure") (HitInfo :type "HitResult Structure (by ref)") (InstigatedBy :type "Controller Object Reference") (DamageCauser :type "Actor Object Reference")))

(event `self.ReceivePointDamage`
  (params (Damage :type "Float (single-precision)") (DamageType :type "DamageType Object Reference") (HitLocation :type "Vector Structure") (HitNormal :type "Vector Structure") (HitComponent :type "PrimitiveComponent Object Reference") (BoneName :type Name) (ShotFromDirection :type "Vector Structure") (InstigatedBy :type "Controller Object Reference") (DamageCauser :type "Actor Object Reference") (HitInfo :type "HitResult Structure (by ref)"))
  (`self.TakeDmage` DamageCauser Damage)
  (`KismetSystemLibrary.DrawDebugSphere` HitLocation 15.0 12 (struct :`R` 1.0 :`G` 0.724107 :`A` 1.0) 0.5 5.0))

(fn `UserConstructionScript`
  (`parent.UserConstructionScript`))