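; BP_AI_Zombie is a zombie AI character that moves between target points while alive.
; On BeginPlay it runs the parent logic, randomizes its IsSimulate flag, waits briefly, then branches on AIModeType.
; In the fixed-point search mode (寻找固定点位模式), it repeatedly moves to the actor from FindTargetPoint, pausing after each success or failure.
; The loop checks the dead state before each move.
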(event `self.ReceiveBeginPlay`
  (`parent.ReceiveBeginPlay`)
  (`self.SetIsSimulate` (`KismetMathLibrary.RandomBool`))
  (`KismetSystemLibrary.Delay` 2.0)
  (switch `EAIModeType` (`self.AIModeType`)
    (:`AIMode_Point`
      (if (not (`self.GetIsDeadState`)) :!label _label
        (bind _movementresult (`|AIMoveTo` self (0.0 0.0 0.0) (`self.FindTargetPoint`))
          (:`OnSuccess`
            _)
          (:`OnFail`
            _))
        (`KismetSystemLibrary.Delay` 1.5)
        (goto _label)))))

(fn `UserConstructionScript`
  (`parent.UserConstructionScript`))